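; Player controller that handles movement and jump input and spawns the player HUD.
; BeginPlay adds the Enhanced Input mapping, caches the character and its movement component, then creates the HUD widget.
; Move input drives the pawn along the controller's forward vector, while jump input sets a held flag.
; Each Tick, BetterJump adds extra gravity while falling or whenever jump is not held, giving variable jump height and faster falls.
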(event `self.ReceiveBeginPlay`
  (bind _returnvalue (`GameplayStatics.GetPlayerCharacter` 0))
  (bind (_returnvalue_x _returnvalue_y _returnvalue_z) (`KismetMathLibrary.BreakVector` (`self.GetVelocity` _returnvalue)))
  (`EnhancedInputSubsystemInterface.AddMappingContext` (pcsubsystem `EnhancedInputLocalPlayerSubsystem` self) "/Game/Input/IMC_Default.IMC_Default" 0 (struct))
  (bind _asbp_player_character (cast `/Game/Blueprints/BP_PlayerCharacter` _returnvalue))
  (set `self.PlayerCharacter` _asbp_player_character)
  (set `self.CharacterMovement` (`Pawn.GetMovementComponent` _asbp_player_character))
  (set `self.PlayerVelocityX` _returnvalue_x)
  (set `self.PlayerVelocityY` _returnvalue_y)
  (set `self.PlayerVelocityZ` _returnvalue_z)
  (`self.SpawnPlayerHUD`))

(event `self.ReceiveTick`
  (params (DeltaSeconds :type "Float (single-precision)"))
  (bind (_returnvalue_x _returnvalue_y _returnvalue_z) (`KismetMathLibrary.BreakVector` (`self.GetVelocity` (`self.PlayerCharacter`))))
  (if (< _returnvalue_z 0.0)
    (`self.BetterJump` DeltaSeconds :!label _label)
    (elif (not (`self.IsJumping`))
      (goto _label))))

(event `EnhancedInput|/Game/Input/IA_Move`
  (params (ActionValue :type "Float (double-precision)") (ElapsedSeconds :type "Float (double-precision)") (TriggeredSeconds :type "Float (double-precision)") (InputAction :type "InputAction Object Reference" :default "/Game/Input/IA_Move.IA_Move"))
  (:`Triggered`
    (`Pawn.AddMovementInput` (`GameplayStatics.GetPlayerPawn` 0) (`self.GetActorForwardVector`) ActionValue false)))

(event `EnhancedInput|/Game/Input/IA_Jump`
  (params (ActionValue :type Boolean) (ElapsedSeconds :type "Float (double-precision)") (TriggeredSeconds :type "Float (double-precision)") (InputAction :type "InputAction Object Reference" :default "/Game/Input/IA_Jump.IA_Jump"))
  (:`Triggered`
    (if (`Character.CanJump` (`self.PlayerCharacter`))
      (set `self.IsJumping` true)
      (`Character.Jump` (`GameplayStatics.GetPlayerCharacter` 0))))
  (:`Completed`
    (set `self.IsJumping` false)))

(fn `BetterJump`
  (params (DeltaTime :type "Float (double-precision)"))
  (bind _charactermovement (`self.CharacterMovement`))
  (bind (_returnvalue_x _returnvalue_y _returnvalue_z) (`KismetMathLibrary.BreakVector` (`self.GetVelocity` (`self.PlayerCharacter`))))
  (set `MovementComponent.Velocity` (`KismetMathLibrary.MakeVector` _returnvalue_x _returnvalue_y (+ _returnvalue_z (* DeltaTime (- (`self.FallMultiplier`) 1.0) (`MovementComponent.GetGravityZ` _charactermovement)))) _charactermovement))

(fn `BetterJumpReleasedTrigger`)

(fn `SpawnPlayerHUD`
  (bind _returnvalue (`|CreateWidget` "/Game/Blueprints/Widget/HUD_Widget.HUD_Widget_C" self))
  (bind _output_get (set `self.HUDWIdgetRef` _returnvalue))
  (`UserWidget.AddToViewport` _output_get 0))

(fn `UserConstructionScript`)